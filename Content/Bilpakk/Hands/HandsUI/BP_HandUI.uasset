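; Hand UI pointer that draws a laser-style beam and an end marker for interacting with widgets.
; Each tick, the end mesh shows only while WidgetPointer is over a hit-test-visible widget and moves to the pointer trace's hit location.
; The beam mesh is stretched along its X scale to the hit distance, or to the full interaction distance when no such widget is hovered.
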(event EventTick
  (params (DeltaSeconds :type Float%20%28single-precision%29))
  (bind _widgetpointer (Variables|Default|GetWidgetPointer))
  (bind _endpointmesh (Variables|Default|GetEndPointMesh))
  (bind _pointermesh (Variables|Default|GetPointerMesh))
  (bind _returnvalue (Class|WidgetInteractionComponent|IsOverHitTestVisibleWidget _widgetpointer))
  (bind (_returnvalue_distance _returnvalue_location) (|PointerTrace _widgetpointer))
  (Rendering|SetVisibility _endpointmesh _returnvalue false)
  (if _returnvalue
    (Transformation|SetWorldLocation _endpointmesh _returnvalue_location false false)
    (Transformation|SetWorldScale3D _pointermesh (Math|Vector|MakeVector _returnvalue_distance 1.0 1.0))
    (else
      (Transformation|SetWorldScale3D _pointermesh (Math|Vector|MakeVector (Variables|/Script/UMG.WidgetInteractionComponent|GetInteractionDistance _widgetpointer) 1.0 1.0)))))

(fn ConstructionScript)