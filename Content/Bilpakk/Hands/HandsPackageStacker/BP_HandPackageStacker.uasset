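; BP_HandPackageStacker is a motion-controller gloved hand for the package stacker.
; On BeginPlay it caches the hand mesh's ABP_GloveGrip animation instance.
; After a short delay, it mirrors the mesh with negative Z scale if the motion source is Left, so one Blueprint handles the left hand too.
; GripStateChanged passes each new grip state to the animation Blueprint.
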(event EventBeginPlay
  (bind _asabp_glove_grip (Utilities|Casting|CastToABP_GloveGrip (Components|SkeletalMesh|GetAnimInstance (Variables|Default|GetHandMesh))))
  (Variables|Default|SetAnim%20BP _asabp_glove_grip)
  (Utilities|FlowControl|Delay 0.2)
  (if (Utilities|Name|Equal(Name) (Variables|/Script/HeadMountedDisplay.MotionControllerComponent|GetMotionSource (Variables|Default|GetMotionControllerComponent)) "Left")
    (Transformation|SetWorldScale3D (Variables|Default|GetHandMesh) "1.000000,1.000000,-1.000000")))

(event Collision|EventActorBeginOverlap
  (params (OtherActor :type Actor%20Object%20Reference)))

(event EventTick
  (params (DeltaSeconds :type Float%20%28single-precision%29)))

(event EventGripStateChanged
  (params (NewState :type EGripState%20Enum :default "Open"))
  (Variables|/Game/Bilpakk/Hands/HandsPackageStacker/SkeletalMeshes/Animations/ABP_GloveGrip.ABP_GloveGrip_C|SetGripState (Variables|Default|GetAnim%20BP) NewState))

(fn ConstructionScript)