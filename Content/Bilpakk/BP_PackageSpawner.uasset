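; BP_PackageSpawner releases three packages in a timed sequence at the start of play in the Bilpakk game.
; BeginPlay waits briefly, runs Setup, then repeatedly fetches the next package and calls its Release with false after a two-second delay.
; The sequence is hardcoded as a linear chain rather than a loop, and Setup and GetNextPackage are called here but defined outside these graphs.
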(event EventBeginPlay
  (Utilities|FlowControl|Delay 0.2)
  (Class|PackageSpawner|Setup)
  (bind _returnvalue (Class|PackageSpawner|GetNextPackage))
  (Utilities|FlowControl|Delay 2.0)
  (Class|PoolActor|Release _returnvalue false)
  (bind _returnvalue_2 (Class|PackageSpawner|GetNextPackage))
  (Utilities|FlowControl|Delay 2.0)
  (Class|PoolActor|Release _returnvalue_2 false)
  (bind _returnvalue_3 (Class|PackageSpawner|GetNextPackage))
  (Utilities|FlowControl|Delay 2.0)
  (Class|PoolActor|Release _returnvalue_3 false))

(event Collision|EventActorBeginOverlap
  (params (OtherActor :type Actor%20Object%20Reference)))

(event EventTick
  (params (DeltaSeconds :type Float%20%28single-precision%29)))

(fn ConstructionScript)